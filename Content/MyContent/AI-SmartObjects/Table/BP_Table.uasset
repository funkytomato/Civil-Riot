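; Table actor that seats an avatar at a nearby Smart Object slot.
; FindSeat searches a box twice the table's bounds for Sit-activity slots, then claims a random result and starts its gameplay behavior through the avatar's AI controller.
; It immediately snaps the avatar to the slot transform without waiting for the behavior to finish, then fires OnFoundSeat.
; If the search fails, it fires OnUnavailable instead.
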(event `FindSeat`
  (params (Avatar :type "Actor Object Reference"))
  (bind (_origin _boxextent) (`self.GetActorBounds` false))
  (set `self.Avatar` Avatar)
  (bind (_outresults _returnvalue) (`SmartObjectSubsystem.FindSmartObjects_BP` (subsystem `SmartObjectSubsystem`) (make `SmartObjectRequest` (`KismetMathLibrary.MakeBoxWithOrigin` _origin (* _boxextent 2.0)) (make `SmartObjectRequestFilter` (struct) "Normal" (struct :`TagDictionary` (struct :`(TagName` "SmartObject.Activity.Sit")) :`QueryTokenStream` "(0,1,1,1,0)" :`AutoDescription` " ANY( SmartObject.Activity.Sit )"))) (`self.Avatar`)))
  (if _returnvalue
    (bind _returnvalue_2 (`SmartObjectBlueprintFunctionLibrary.MarkSmartObjectSlotAsClaimed` (`.SlotHandle` (break `SmartObjectRequestResult` (`KismetArrayLibrary.Array_Random` _outresults))) (`self.Avatar`)))
    (`AITask_UseGameplayBehaviorSmartObject.UseSmartObjectWithGameplayBehavior` (`AIBlueprintHelperLibrary.GetAIController` (`self.Avatar`)) _returnvalue_2
      (:`then`
        (`self.K2_SetActorLocationAndRotation` (`self.Avatar`) (.location (`SmartObjectSubsystem.GetSlotTransform` (subsystem `SmartObjectSubsystem`) _returnvalue_2)) (.rotation (`SmartObjectSubsystem.GetSlotTransform` (subsystem `SmartObjectSubsystem`) _returnvalue_2)) false false)
        (`self.OnFoundSeat` (`self.Avatar`))))
    (else
      (`self.OnUnavailable` (`self.Avatar`)))))

(fn `UserConstructionScript`)