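; BP_NPC_Friendly is a friendly NPC that can be ordered to move to a location.
; CommandMoveto ignores zero vectors, otherwise runs BT_CommandMoveTo on its AI controller and writes the target to the TargetLocation blackboard key.
; CommandComplete stops the controller's brain logic without starting another tree.
; A call to run BT_Wander is present but unconnected, and BeginPlay only calls its parent.
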(event `self.ReceiveBeginPlay`
  (`parent.ReceiveBeginPlay`))

(event `/Game/MyContent/Ai/BPI_AI.CommandMoveTo`
  (params (Location :type "Vector Structure"))
  (if (!= (`KismetMathLibrary.VSize` Location) 0.0)
    (`AIController.RunBehaviorTree` (`AIBlueprintHelperLibrary.GetAIController` self) "/Game/MyContent/Ai/BT_CommandMoveTo.BT_CommandMoveTo")
    (`BlackboardComponent.SetValueAsVector` (`AIBlueprintHelperLibrary.GetBlackboard` null) "TargetLocation" Location)))

(event `/Game/MyContent/Ai/BPI_AI.CommandComplete`
  (`BrainComponent.StopLogic` (`AIController.BrainComponent` (`AIBlueprintHelperLibrary.GetAIController` self)) ""))

(fn `UserConstructionScript`
  (`parent.UserConstructionScript`))