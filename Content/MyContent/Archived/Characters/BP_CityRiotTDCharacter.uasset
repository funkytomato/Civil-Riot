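; Top-down character for CityRiotTD with click-to-interact, a death state and a fixed attack range.
; Clicking it sets it as the player character's interact target; Tick fires the interact message once that target is close, then clears it and stops movement.
; When interacted with, it makes the interacting character jump.
; OnDead flags death and stops movement; a smoothed turn toward the controller's cached destination exists but is never run.
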(event `self.ReceiveBeginPlay`
  (bind _asbp_city_riot_tdcontroller (cast `/Game/MyContent/Archived/Characters/BP_CityRiotTDController` (`GameplayStatics.GetPlayerController` 0)))
  (set `self.As BP Top Down Controller` _asbp_city_riot_tdcontroller))

(event `self.ReceiveTick`
  (params (DeltaSeconds :type "Float (single-precision)"))
  (bind _currentinteracttarget (`self.CurrentInteractTarget`)
    (:`then`
      (if (<= (`self.GetDistanceTo` _currentinteracttarget self) 150.0)
        (message `/Game/MyContent/AI/Blueprints/I_InteractInterface.InteractWith` (`self.CurrentInteractTarget`) self)
        (set `self.CurrentInteractTarget` null)
        (`MovementComponent.StopMovementImmediately` (`self.CharacterMovement`))))
    (:`else`)))

(event `/Game/MyContent/AI/Blueprints/I_InteractInterface.SetInteractTarget`
  (params (Actor :type "Actor Object Reference"))
  (bind _output_get (set `self.CurrentInteractTarget` Actor))
  (`KismetSystemLibrary.PrintString` (`KismetSystemLibrary.GetDisplayName` _output_get)))

(event `OnDead`
  (set `self.IsDead?` true)
  (`NavMovementComponent.StopActiveMovement` (`self.CharacterMovement`)))

(event `self.ReceiveActorOnClicked`
  (params (ButtonPressed :type "Key Structure"))
  (message `/Game/MyContent/AI/Blueprints/I_InteractInterface.SetInteractTarget` (`GameplayStatics.GetPlayerCharacter` 0) self))

(event `/Game/MyContent/AI/Blueprints/I_InteractInterface.InteractWith`
  (params (Character :type "Character Object Reference"))
  (`self.Jump` Character))

(fn `GetAttackRange`
  (returns (Range :type "Float (double-precision)"))
  (return 300.0))

(fn `LookAtDestination`
  (bind (_returnvalue_roll _returnvalue_pitch _returnvalue_yaw) (`KismetMathLibrary.BreakRotator` (`KismetMathLibrary.FindLookAtRotation` (`self.K2_GetActorLocation`) (`/Game/MyContent/Archived/Characters/BP_CityRiotTDController.CachedDestination` (`self.As BP Top Down Controller`)))))
  (`self.K2_SetActorRotation` (`KismetMathLibrary.RInterpTo` (`self.K2_GetActorRotation`) (`KismetMathLibrary.MakeRotator` 0.0 0.0 _returnvalue_yaw) (`GameplayStatics.GetWorldDeltaSeconds`) 3.0)))

(fn `UserConstructionScript`)