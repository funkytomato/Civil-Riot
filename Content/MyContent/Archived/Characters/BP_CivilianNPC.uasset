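; BP_CivilianNPC is an AI-controlled civilian character that can interact with targets, be interacted with, and act as a dealer.
; On Tick it checks distance to its interact target, then sends the interaction, clears the target and stops moving when close.
; Interacting with it makes the other character jump.
; Dealer events toggle a wares-for-sale flag, death sets a flag, and attack range is fixed.
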(event `self.ReceiveBeginPlay`
  ;[1 1 1] BeginPlay - Set AIController Reference
  (bind _asnpc_aicontroller (cast `/Game/MyContent/Archived/Characters/NPC_AIController` (`AIBlueprintHelperLibrary.GetAIController` null)))
  (set `self.NPCAIControllerRef` _asnpc_aicontroller))

(event `OfferWares`
  (set `self.ReadyToSellWares` true))

(event `StopOfferingWares`
  (set `self.ReadyToSellWares` false))

(event `self.ReceiveTick`
  (params (DeltaSeconds :type "Float (single-precision)"))
  ;[1 1 1] OnTick - Check for Interaction Actor
  (bind _currentinteracttarget (`self.CurrentInteractTarget`)
    (:`then`
      (if (<= (`self.GetDistanceTo` _currentinteracttarget self) 150.0)
        (message `/Game/MyContent/AI/Blueprints/I_InteractInterface.InteractWith` (`self.CurrentInteractTarget`) self)
        (set `self.CurrentInteractTarget` null)
        (`MovementComponent.StopMovementImmediately` (`self.CharacterMovement`))))
    (:`else`)))

(event `/Game/MyContent/AI/Blueprints/I_InteractInterface.SetInteractTarget`
  (params (Actor :type "Actor Object Reference"))
  ;[1 1 1] Interface Interaction Events
  (bind _output_get (set `self.CurrentInteractTarget` Actor))
  (`KismetSystemLibrary.PrintString` (`KismetSystemLibrary.GetDisplayName` _output_get)))

(event `self.ReceiveActorOnClicked`
  (params (ButtonPressed :type "Key Structure"))
  ;[1 1 1] Interface Interaction Events
)

(event `/Game/MyContent/AI/Blueprints/I_InteractInterface.InteractWith`
  (params (Character :type "Character Object Reference"))
  ;[1 1 1] Interface Interaction Events
  (`self.Jump` Character))

(event `OnDead`
  (set `self.IsDead?` true))

(fn `GetAttackRange`
  (returns (Range :type "Float (double-precision)"))
  (return 300.0))

(fn `UserConstructionScript`)