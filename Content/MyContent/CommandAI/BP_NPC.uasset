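; NPC character for command AI, with team tag, death flag, overhead-style stats widget and click-to-interact behavior.
; Stat update functions route Health, Stamina, Morale and Temperament changes through a stats component, while attack range is stubbed at zero.
; Through I_InteractionInterface, clicks make it the player's target, and interacting makes the instigator jump.
; Tick triggers interaction and halts movement near CurrentInteractTarget, though SetInteractTarget only clears that variable.
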(event `self.ReceiveBeginPlay`
  (bind _aswbp_stats (cast `/Game/MyContent/UI/WBP_Stats` (`WidgetComponent.GetWidget` (`self.Widget`))))
  (set `/Game/MyContent/UI/WBP_Stats.OwnerRef` self _aswbp_stats))

(event `OnDead`
  (set `self.IsDead?` true))

(event `/Game/MyContent/CommandAI/BPI_AI.SetTeam`
  (params (TeamTag :type "GameplayTag Structure"))
  (set `self.Team Tag` TeamTag))

(event `/Game/MyContent/AI/Blueprints/I_InteractInterface.SetInteractTarget`
  (params (Actor :type "Actor Object Reference"))
  ; Interaction Interface Events - I_InteractionInterface
  (bind _output_get (set `self.CurrentInteractTarget` null))
  (`KismetSystemLibrary.PrintString` (`KismetSystemLibrary.GetDisplayName` _output_get)))

(event `self.ReceiveActorOnClicked`
  (params (ButtonPressed :type "Key Structure"))
  ; Interaction Interface Events - I_InteractionInterface
  (message `/Game/MyContent/AI/Blueprints/I_InteractInterface.SetInteractTarget` (`GameplayStatics.GetPlayerCharacter` 0) self))

(event `/Game/MyContent/AI/Blueprints/I_InteractInterface.InteractWith`
  (params (Character :type "Character Object Reference"))
  ; Interaction Interface Events - I_InteractionInterface
  (`self.Jump` Character))

(event `self.ReceiveTick`
  (params (DeltaSeconds :type "Float (single-precision)"))
  ; Interaction Interface Events - I_InteractionInterface
  (bind _currentinteracttarget (`self.CurrentInteractTarget`)
    (:`then`
      (if (<= (`self.GetDistanceTo` _currentinteracttarget self) 150.0)
        (message `/Game/MyContent/AI/Blueprints/I_InteractInterface.InteractWith` (`self.CurrentInteractTarget`) self)
        (set `self.CurrentInteractTarget` null)
        (`MovementComponent.StopMovementImmediately` (`self.CharacterMovement`))))
    (:`else`)))

(fn `GetAttackRange`
  (returns (Range :type "Float (double-precision)"))
  (return 0.0))

(fn `GetTeam`
  (returns (TeamTag :type "GameplayTag Structure"))
  (return (`self.Team Tag`)))

(fn `UpdateHealth`
  (params (amount :type "Float (double-precision)"))
  (returns (Health :type "Float (double-precision)"))
  (bind (_statdepleted _currentvalue) (`/Game/MyContent/AI/Systems/StatsComponentNew.AlterStat` (`self.StatsComponentNew`) "Health" amount))
  (return _currentvalue))

(fn `UpdateMorale`
  (params (amount :type "Float (double-precision)"))
  (returns (Morale :type "Float (double-precision)"))
  (bind (_statdepleted _currentvalue) (`/Game/MyContent/AI/Systems/StatsComponentNew.AlterStat` (`self.StatsComponentNew`) "Morale" amount))
  (return _currentvalue))

(fn `UpdateStamina`
  (params (amount :type "Float (double-precision)"))
  (returns (Stamina :type "Float (double-precision)"))
  (bind (_statdepleted _currentvalue) (`/Game/MyContent/AI/Systems/StatsComponentNew.AlterStat` (`self.StatsComponentNew`) "Stamina" amount))
  (return _currentvalue))

(fn `UpdateTemperament`
  (params (amount :type "Float (double-precision)"))
  (returns (Temperament :type "Float (double-precision)"))
  (bind (_statdepleted _currentvalue) (`/Game/MyContent/AI/Systems/StatsComponentNew.AlterStat` (`self.StatsComponentNew`) "Temperament" amount))
  (return _currentvalue))

(fn `UserConstructionScript`)